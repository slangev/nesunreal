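; GameBP is an actor that displays a DrawingCanvasBP's dynamic texture as the player's view.
; On BeginPlay it switches to unlit view mode, makes itself the view target, and creates the drawing canvas object at the configured pixel size.
; It feeds that texture into a dynamic material on the Canvas component, then scales the component and sets the camera's ortho width.
; Each frame it ticks the drawing canvas.
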(event EventBeginPlay
  (Development|ExecuteConsoleCommand "viewmode unlit" 0)
  (Game|Player|SetViewTargetwithBlend (Game|GetPlayerController 0) self 0.0 "VTBlend_Linear" 0.0 false) ; Setup Camera
  (CallFunction|InitializeDrawingCanvas))

(event EventTick
  (params (DeltaSeconds :type Float%20%28single-precision%29))
  (CallFunction|TickRender))

(fn ConstructionScript)

(fn InitializeDrawingCanvas
  ;[0 0.02604 0.01004] Init Drawing Canvas Object
  (bind _returnvalue (Game|ConstructObjectfromClass "/Game/Blueprints/DrawingCanvasBP.DrawingCanvasBP_C" self))
  (Variables|Default|SetDrawingCanvas _returnvalue)
  (Class|DrawingCanvas|InitializeCanvas (Variables|Default|GetDrawingCanvas) (Variables|Default|GetCanvasWidth) (Variables|Default|GetCanvasHeight))
  ;[0 0.01121 0.04167] Init Drawing Canvas Material
  (bind _returnvalue_2 (Rendering|Material|CreateDynamicMaterialInstance (Variables|Default|GetCanvas) 0 0 "None" :!class /Script/Engine.PrimitiveComponent))
  (Variables|Default|SetCanvasMID _returnvalue_2)
  (Rendering|Material|SetTextureParameterValue (Variables|Default|GetCanvasMID) "TextureInput" (Variables|/Script/Tutorial_Canvas.DrawingCanvas|GetdynamicCanvas (Variables|Default|GetDrawingCanvas)))
  ;[0 0.01121 0.04167] Init Scene Objects
  (Transformation|SetRelativeScale3D (Variables|Default|GetCanvas) (Math|Vector|MakeVector 2.5 1.1 0.0))
  (Class|CameraComponent|SetOrthoWidth (Variables|Default|GetCamera) (Math|Conversions|ToFloat(Integer) (Variables|Default|GetCanvasWidth))))

(fn TickRender
  (bind _output_get (Variables|Default|SetDrawingCanvas (Variables|Default|GetDrawingCanvas)))
  (Class|DrawingCanvas|Tick _output_get))